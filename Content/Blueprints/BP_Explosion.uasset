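; BP_Explosion is a one-shot explosion actor that damages the player and destroys itself, with all logic in BeginPlay.
; A sphere overlap around its location looks for WorldDynamic and Pawn objects, applying fixed damage only to the player pawn as BP_ThirdPersonCharacter.
; It then spawns the scaled-up P_Explosion effect and plays BP_CamShake as a world camera shake with a very large outer radius.
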(event EventBeginPlay
  (bind _returnvalue (Game|Player|GetPlayerPawn 0))
  (bind _outactors (Collision|SphereOverlapActors (Transformation|GetActorLocation) 3e+02 (Utilities|Array|MakeArray "ObjectTypeQuery2" "ObjectTypeQuery3") 0))
  (for _array_element _outactors
    (if (== _array_element _returnvalue)
      (bind _asbp_third_person_character (Utilities|Casting|CastToBP_ThirdPersonCharacter _returnvalue))
      (Game|Damage|ApplyDamage _asbp_third_person_character 1e+01 0 0)))
  (Niagara|SpawnSystematLocation "/Game/P_Explosion.P_Explosion" (Transformation|GetActorLocation) "0, 0, 0" "3.000000,3.000000,3.000000")
  (Camera|PlayWorldCameraShake "/Game/Blueprints/BP_CamShake.BP_CamShake_C" (Transformation|GetActorLocation) 1e+02 1e+08)
  (Actor|DestroyActor))

(fn ConstructionScript)