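; Arena handler actor that plays a short camera intro when the player pawn overlaps its StartCollision trigger.
; It disables player input and snaps the third-person character's FollowCamera to two viewpoint components in turn, holding each for a few seconds.
; It then resets the camera's relative transform and restores input.
; Nothing guards against retriggering on a later overlap.
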(event OnComponentBeginOverlap(StartCollision)
  (params (OverlappedComponent :type Primitive%20Component%20Object%20Reference) (OtherActor :type Actor%20Object%20Reference) (OtherComp :type Primitive%20Component%20Object%20Reference) (OtherBodyIndex :type Integer) (bFromSweep :type Boolean) (SweepResult :type Hit%20Result%20Structure%20%28by%20ref%29))
  (bind _returnvalue (Game|Player|GetPlayerPawn 0))
  (if (== OtherActor _returnvalue)
    (Input|DisableInput _returnvalue (Game|GetPlayerController 0))
    (bind _asbp_third_person_character (Utilities|Casting|CastToBP_ThirdPersonCharacter _returnvalue))
    (Transformation|SetWorldTransform (Variables|/Game/ThirdPerson/Blueprints/BP_ThirdPersonCharacter.BP_ThirdPersonCharacter_C|GetFollowCamera _asbp_third_person_character) (Transformation|GetWorldTransform (Variables|Default|GetPOV1)) false false)
    (Utilities|FlowControl|Delay 3.0)
    (Transformation|SetWorldTransform (Variables|/Game/ThirdPerson/Blueprints/BP_ThirdPersonCharacter.BP_ThirdPersonCharacter_C|GetFollowCamera _asbp_third_person_character) (Transformation|GetWorldTransform (Variables|Default|GetPOV2)) false false)
    (Utilities|FlowControl|Delay 5.0)
    (Transformation|SetRelativeTransform (Variables|/Game/ThirdPerson/Blueprints/BP_ThirdPersonCharacter.BP_ThirdPersonCharacter_C|GetFollowCamera _asbp_third_person_character) (Math|Transform|MakeTransform "0, 0, 0" "0, 0, 0" "1.000000,1.000000,1.000000") false false)
    (Input|EnableInput (Game|Player|GetPlayerPawn 0) (Game|GetPlayerController 0))))

(fn ConstructionScript)