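; BP_Elevator is an elevator that moves a cube between a bottom point and a top point, starting on BeginPlay with no trigger.
; A timeline's alpha lerps between the two points' world locations to set the cube's position without sweep.
; Each time the timeline finishes, it calls MoveElevator again, where a FlipFlop alternates play and reverse-from-end for endless back-and-forth travel.
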(event Custom|MoveElevator
  (Utilities|FlowControl|FlipFlop
    (:A
      (bind _alpha (Timeline|ElevatorTimeline Play)
        (:Update
          (Transformation|SetWorldLocation (Variables|Default|GetElevatorCube) (Math|Vector|Lerp(Vector) (Transformation|GetWorldLocation (Variables|Default|GetBottomPoint)) (Transformation|GetWorldLocation (Variables|Default|GetTopPoint)) _alpha) false false))
        (:Finished
          (CallFunction|MoveElevator))))
    (:B
      (Timeline|ElevatorTimeline ReverseFromEnd))))

(event EventBeginPlay
  (CallFunction|MoveElevator))

(fn ConstructionScript)