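; Frog enemy character that alternates between hopping to face the player and leaping at them, and is destroyed on death.
; A looping MultiGate runs a timeline-driven reorient, then a jump and delayed launch toward the player, each after a randomized cooldown.
; During the leap its coating overlaps pawns and box overlaps damage and knock back the player.
; Tick detects standstill, restores blocking, spawns an explosion and resumes the cycle.
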(event Death(AC_Health)
  (Actor|DestroyActor))

(event OnComponentBeginOverlap(Box)
  (params (OverlappedComponent :type Primitive%20Component%20Object%20Reference) (OtherActor :type Actor%20Object%20Reference) (OtherComp :type Primitive%20Component%20Object%20Reference) (OtherBodyIndex :type Integer) (bFromSweep :type Boolean) (SweepResult :type Hit%20Result%20Structure%20%28by%20ref%29))
  (bind _returnvalue (Game|Player|GetPlayerPawn 0))
  (if (and (== OtherActor _returnvalue) (Variables|Default|GetCollisionDamageActive))
    (bind _asbp_third_person_character (Utilities|Casting|CastToBP_ThirdPersonCharacter _returnvalue))
    (Game|Damage|ApplyDamage _returnvalue (Variables|Default|GetCollisionDamage) 0 0)
    (Character|LaunchCharacter _asbp_third_person_character (Math|Vector|RotateVector (Math|Vector|RotateVector (Variables|Default|GetKnockback) (Math|Rotator|FindLookatRotation (Transformation|GetActorLocation) (Transformation|GetActorLocation _returnvalue))) "0, 0, 0") false false)))

(event Custom|Reorient
  (Variables|Default|SetLocationStore (Transformation|GetActorLocation))
  (bind (_direction _alpha _alpharotation) (Timeline|Timeline PlayFromStart)
    (:Update
      (Transformation|SetActorLocation (Math|Vector|MakeVector (.x (Variables|Default|GetLocationStore)) (.y (Variables|Default|GetLocationStore)) (+ (.z (Variables|Default|GetLocationStore)) (Math|Float|Lerp 0.0 1.5e+02 _alpha))) false false)
      (Transformation|SetActorRotation (Math|Rotator|Lerp(Rotator) (Transformation|GetActorRotation) (Math|Rotator|FindLookatRotation (Transformation|GetActorLocation) (Transformation|GetActorLocation (Game|Player|GetPlayerPawn 0))) _alpharotation true)))
    (:Finished
      (CallFunction|PickAction))))

(event Custom|PickAction
  (Utilities|FlowControl|MultiGate false true -1
    (:Out%200
      (Utilities|FlowControl|Delay (Variables|Default|GetCooldownTime))
      (CallFunction|Reorient)
      (Variables|Default|SetCooldownTime (+ (Math|Random|RandomFloatinRange -0.5 0.5) 1.0)))
    (:Out%201
      (Utilities|FlowControl|Delay (Variables|Default|GetCooldownTime))
      (CallFunction|JumpAttack)
      (Variables|Default|SetCooldownTime (+ (Math|Random|RandomFloatinRange -0.5 0.5) 5.0)))))

(event Custom|JumpAttack
  (Character|Jump)
  (Development|PrintString "Jump!")
  (Utilities|FlowControl|Delay 2.0)
  (Components|Movement|StopMovementImmediately (Variables|Character|GetCharacterMovement))
  (Character|StopJumping)
  (Character|LaunchCharacter (* (- (Transformation|GetActorLocation (Game|Player|GetPlayerPawn 0)) (Transformation|GetActorLocation)) 1.05) true true)
  (Variables|Default|SetWaitForStandstill true)
  (Variables|Default|SetCollisionDamageActive true)
  (Collision|SetCollisionResponsetoChannel (Variables|Default|GetCoating) "ECC_Pawn" "ECR_Overlap"))

(event EventBeginPlay
  (CallFunction|PickAction))

(event EventTick
  (params (DeltaSeconds :type Float%20%28single-precision%29))
  (if (Variables|Default|GetWaitForStandstill)
    (if (<= (Math|Vector|VectorLength (Variables|/Script/Engine.MovementComponent|GetVelocity (Variables|Character|GetCharacterMovement))) 0.1)
      (Development|PrintString "HERE!")
      (Variables|Default|SetWaitForStandstill false)
      (CallFunction|PickAction)
      (Variables|Default|SetCollisionDamageActive false)
      (Collision|SetCollisionResponsetoChannel (Variables|Default|GetCoating) "ECC_Pawn" "ECR_Block")
      (Game|SpawnActorfromClass "/Game/Blueprints/BP_Explosion.BP_Explosion_C" (Transformation|GetActorTransform) "Undefined" "MultiplyWithRoot" 0 0))))

(fn ConstructionScript)