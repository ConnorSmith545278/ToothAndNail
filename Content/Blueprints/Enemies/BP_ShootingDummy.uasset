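; BP_ShootingDummy is an enemy that starts firing energy balls when the player pawn first overlaps its StartAttacking trigger.
; That one-time trigger starts a looping timer, with a negative start delay for a quicker first volley, and registers the death handler with ACHealth.
; Each volley spawns three staggered BP_EnergyBall actors at offsets above the dummy.
; On death, it destroys itself and clears the timer.
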(event OnComponentBeginOverlap(StartAttacking)
  (params (OverlappedComponent :type Primitive%20Component%20Object%20Reference) (OtherActor :type Actor%20Object%20Reference) (OtherComp :type Primitive%20Component%20Object%20Reference) (OtherBodyIndex :type Integer) (bFromSweep :type Boolean) (SweepResult :type Hit%20Result%20Structure%20%28by%20ref%29))
  (if (== OtherActor (Game|Player|GetPlayerPawn 0))
    (Utilities|FlowControl|DoOnce false
      (:Completed
        (bind _returnvalue (Utilities|Time|SetTimerbyEvent (delegate Custom|SpawnProjectiles) 2.9 true false -2.0))
        (EventDispatchers|AssignDeath (Variables|Default|GetAC_Health) (delegate Custom|Death_Event))))))

(event Custom|SpawnProjectiles
  (Game|SpawnActorfromClass "/Game/Blueprints/BP_EnergyBall.BP_EnergyBall_C" (Math|Transform|MakeTransform (+ (Transformation|GetActorLocation) "0.000000,0.000000,200.000000") "0, 0, 0" "1.000000,1.000000,1.000000") "Undefined" "MultiplyWithRoot" 0 0)
  (Utilities|FlowControl|Delay 0.3)
  (Game|SpawnActorfromClass "/Game/Blueprints/BP_EnergyBall.BP_EnergyBall_C" (Math|Transform|MakeTransform (+ (Transformation|GetActorLocation) "100.000000,0.000000,100.000000") "0, 0, 0" "1.000000,1.000000,1.000000") "Undefined" "MultiplyWithRoot" 0 0)
  (Utilities|FlowControl|Delay 0.3)
  (Game|SpawnActorfromClass "/Game/Blueprints/BP_EnergyBall.BP_EnergyBall_C" (Math|Transform|MakeTransform (+ (Transformation|GetActorLocation) "-100.000000,0.000000,100.000000") "0, 0, 0" "1.000000,1.000000,1.000000") "Undefined" "MultiplyWithRoot" 0 0))

(event Custom|Death_Event
  (Actor|DestroyActor)
  (Utilities|Time|ClearandInvalidateTimerbyHandle (stale OnComponentBeginOverlap(StartAttacking) _returnvalue)))

(fn ConstructionScript)