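; Spore frog enemy that alternates between a hop to turn toward the player and a leaping dive attack.
; A looping MultiGate in PickAction sequences the two moves with cooldown delays, and each move calls PickAction when finished.
; Timelines drive all movement; the attack rises, pauses, then sweeps toward the player's captured position.
; Box overlaps during the dive damage and launch the player, and AC_Health death destroys the frog.
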(event Death(AC_Health)
  (Actor|DestroyActor))

(event OnComponentBeginOverlap(Box)
  (params (OverlappedComponent :type Primitive%20Component%20Object%20Reference) (OtherActor :type Actor%20Object%20Reference) (OtherComp :type Primitive%20Component%20Object%20Reference) (OtherBodyIndex :type Integer) (bFromSweep :type Boolean) (SweepResult :type Hit%20Result%20Structure%20%28by%20ref%29))
  (bind _returnvalue (Game|Player|GetPlayerPawn 0))
  (if (and (== OtherActor _returnvalue) (Variables|Default|GetCollisionDamageActive))
    (bind _asbp_third_person_character (Utilities|Casting|CastToBP_ThirdPersonCharacter _returnvalue))
    (Game|Damage|ApplyDamage _returnvalue (Variables|Default|GetCollisionDamage) 0 0)
    (Character|LaunchCharacter _asbp_third_person_character (Math|Vector|RotateVector (Math|Vector|RotateVector (Variables|Default|GetKnockback) (Math|Rotator|FindLookatRotation (Transformation|GetActorLocation) (Transformation|GetActorLocation _returnvalue))) "0, 0, 0") false false)
    (elif (== (Utilities|GetClass OtherActor) "BP_SporeFrog_C")
      _)))

(event Custom|Reorient
  (Variables|Default|SetLocationStore (Transformation|GetActorLocation))
  (bind (_direction _alpha _alpharotation) (Timeline|Alpha PlayFromStart)
    (:Update
      (Transformation|SetActorLocation (Math|Vector|MakeVector (.x (Variables|Default|GetLocationStore)) (.y (Variables|Default|GetLocationStore)) (+ (.z (Variables|Default|GetLocationStore)) (Math|Float|Lerp 0.0 1.5e+02 _alpha))) false false)
      (Transformation|SetActorRotation (Math|Rotator|Lerp(Rotator) (Transformation|GetActorRotation) (Math|Rotator|FindLookatRotation (Transformation|GetActorLocation) (Transformation|GetActorLocation (Game|Player|GetPlayerPawn 0))) _alpharotation true)))
    (:Finished
      (CallFunction|PickAction))))

(event Custom|PickAction
  (Utilities|FlowControl|MultiGate false true -1
    (:Out%200
      (Utilities|FlowControl|Delay (Variables|Default|GetCooldownTime))
      (CallFunction|Reorient)
      (Variables|Default|SetCooldownTime 1.0))
    (:Out%201
      (Utilities|FlowControl|Delay (Variables|Default|GetCooldownTime))
      (CallFunction|JumpAttack)
      (Variables|Default|SetCooldownTime 5.0))))

(event Custom|JumpAttack
  (Variables|Default|SetLocationStore (Transformation|GetActorLocation))
  (bind _newtrack_0 (Timeline|JumpUp PlayFromStart)
    (:Update
      (Transformation|SetActorLocation (Math|Vector|MakeVector (.x (Variables|Default|GetLocationStore)) (.y (Variables|Default|GetLocationStore)) (+ (.z (Variables|Default|GetLocationStore)) (Math|Float|Lerp (.z (Variables|Default|GetLocationStore)) 1.5e+03 _newtrack_0))) false false))
    (:Finished
      (Utilities|FlowControl|Delay 0.3)
      (bind _output_get (Variables|Default|SetLocationStore (Transformation|GetActorLocation)))
      (bind _output_get_2 (Variables|Default|SetTargetLocation (Transformation|GetActorLocation (Game|Player|GetPlayerPawn 0))))
      (Variables|Default|SetCollisionDamageActive true)
      (bind _newtrack_0_2 (Timeline|Timeline PlayFromStart)
        (:Update
          (Transformation|SetActorLocation (Math|Vector|Lerp(Vector) (Variables|Default|GetLocationStore) _output_get_2 _newtrack_0_2) true false)
          (Transformation|SetActorRotation (Math|Rotator|MakeRotator 0.0 0.0 (.yaw (Math|Rotator|Lerp(Rotator) (Transformation|GetActorRotation) (Math|Rotator|FindLookatRotation _output_get _output_get_2) _newtrack_0_2)))))
        (:Finished
          (Variables|Default|SetCollisionDamageActive false)
          (CallFunction|PickAction))))))

(event EventBeginPlay
  (CallFunction|PickAction))

(fn ConstructionScript)