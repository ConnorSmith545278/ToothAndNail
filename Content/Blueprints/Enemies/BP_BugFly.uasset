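; BP_BugFly is a flying bug enemy that travels between bug spots and is destroyed when its health component reports death.
; MoveToBugSpot stores its current location, takes the given spot as target and turns to face it.
; Each tick it moves toward the target at constant speed without sweeping and, once very close, notifies its BugHandler that it has arrived.
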(event Death(AC_Health)
  (Actor|DestroyActor))

(event Custom|MoveToBugSpot
  (params (ActiveBugSpot :type BP%20Bug%20Target%20Spot%20Object%20Reference))
  (Variables|Default|SetPrevious%20Location (Transformation|GetActorLocation))
  (bind _output_get (Variables|Default|SetTarget%20Location (Transformation|GetActorLocation ActiveBugSpot)))
  (Transformation|SetActorRotation (Math|Rotator|FindLookatRotation (Transformation|GetActorLocation) _output_get)))

(event EventTick
  (params (DeltaSeconds :type Float%20%28single-precision%29))
  (Transformation|SetActorLocation (Math|Interpolation|VInterptoConstant (Transformation|GetActorLocation) (Variables|Default|GetTarget%20Location) DeltaSeconds (Variables|Default|GetSpeed)) false false)
  (if (< (Math|Vector|Distance(Vector) (Transformation|GetActorLocation) (Variables|Default|GetTarget%20Location)) 3.0)
    (Default|BugArrived (Variables|Default|GetBugHandler) self)))

(fn ConstructionScript)