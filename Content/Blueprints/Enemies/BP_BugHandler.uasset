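; BP_BugHandler spawns a group of BP_BugFly enemies and directs them between BP_BugTargetSpot actors in the level.
; On BeginPlay it gathers the spots, picks a random active one, and starts a looping timer that spawns flies at its location until BugCount is reached.
; Each fly gets a handler reference, an AI controller and the shared active spot.
; BugArrived re-rolls that spot and redirects only the arriving fly.
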(event Custom|SpawnBug
  (bind _bugstospawn (Variables|Default|GetBugsToSpawn))
  (if (> _bugstospawn 0)
    (Math|Integer|DecrementInt _bugstospawn
      (:%20%20
        (bind _returnvalue (Game|SpawnActorfromClass "/Game/Blueprints/Enemies/BP_BugFly.BP_BugFly_C" (Transformation|GetActorTransform) "AlwaysSpawn" "MultiplyWithRoot" 0 0))
        (Variables|/Game/Blueprints/Enemies/BP_BugFly.BP_BugFly_C|SetBugHandler _returnvalue self)
        (Utilities|Array|Add (Variables|Default|GetBugs) _returnvalue)
        (CallFunction|AssignBugSpot _returnvalue)
        (Pawn|SpawnDefaultController _returnvalue)))
    (else
      (Utilities|Time|ClearandInvalidateTimerbyHandle (stale EventBeginPlay _returnvalue)))))

(event Custom|AssignBugSpot
  (params (Bug :type BP%20Bug%20Fly%20Object%20Reference))
  (Default|MovetoBugSpot Bug (Variables|Default|GetActiveBugSpot)))

(event Custom|BugArrived
  (params (Bug :type BP%20Bug%20Fly%20Object%20Reference))
  (Variables|Default|SetActiveBugSpot (.OutItem (Utilities|Array|Random (Variables|Default|GetBugSpots))))
  (CallFunction|AssignBugSpot Bug))

(event EventBeginPlay
  (Utilities|FlowControl|Sequence
    (:then_0
      (Variables|Default|SetBugsToSpawn (Variables|Default|GetBugCount)))
    (:then_1
      (bind _outactors (Actor|GetAllActorsOfClass "/Game/Blueprints/Enemies/BP_BugTargetSpot.BP_BugTargetSpot_C"))
      (bind _output_get (Variables|Default|SetBugSpots _outactors))
      (Variables|Default|SetActiveBugSpot (.OutItem (Utilities|Array|Random _output_get))))
    (:then_2
      (bind _returnvalue (Utilities|Time|SetTimerbyEvent (delegate Custom|SpawnBug) 0.5 true)))))

(fn ConstructionScript)