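; AC_Health is an actor component that tracks its owner's health and reacts to hammer hits.
; CurrentHealth starts at MaxHealth, and LoseHealth subtracts damage, printing either the remaining health or a death message with no further death handling.
; OnHammerHit walks the owner's directly attached actors in reverse and sends RipNailMessage, passing itself, to each BP_StuckNail child.
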(event Custom|LoseHealth
  (params (HealthLost :type Float%20%28double-precision%29))
  ;[0.15 0.15 0.15 0.5] basic losing health
  (bind _output_get (Variables|Default|SetCurrentHealth (- (Variables|Default|GetCurrentHealth) HealthLost)))
  (if (<= _output_get 0.0)
    (Development|PrintString "Dead!!!")
    (else
      (Development|PrintString (Utilities|String|Append "Health left: " (Utilities|String|ToString(Float) _output_get))))))

(event EventOnHammerHit
  (bind _returnvalue (Components|GetOwner))
  (bind _outactors (Actor|GetAttachedActors _returnvalue true false))
  ;[0.15 0.15 0.15 0.5] Event that triggers when the hammer hits the opponent
  (bind _output_get (Variables|Default|SetRippedNailCounter (Utilities|Array|Length _outactors)))
  (while (> _output_get 0)
    (Math|Integer|DecrementInt (Variables|Default|GetRippedNailCounter)
      (:%20%20
        (if (Utilities|ClassIsChildOf (Utilities|GetClass (Utilities|Array|Get(acopy) _outactors (Variables|Default|GetRippedNailCounter))) "/Game/Blueprints/BP_StuckNail.BP_StuckNail_C")
          (Class|BPINailRip|RipNail(Message) (Utilities|Array|Get(acopy) _outactors (Variables|Default|GetRippedNailCounter)) self))))))

(event EventBeginPlay
  (Variables|Default|SetCurrentHealth (Variables|Default|GetMaxHealth)))