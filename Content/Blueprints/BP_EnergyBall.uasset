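; BP_EnergyBall is a delayed-launch projectile that fires at the player and damages them on contact.
; One second after BeginPlay it turns toward player pawn 0, then activates ProjectileMovement along local X at its initial speed, with no further re-aiming in the graph.
; When the Ball component overlaps an exact BP_ThirdPersonCharacter, a DoOnce-guarded branch applies damage, spawns an explosion effect and destroys the actor.
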(event OnComponentBeginOverlap(Ball)
  (params (OverlappedComponent :type Primitive%20Component%20Object%20Reference) (OtherActor :type Actor%20Object%20Reference) (OtherComp :type Primitive%20Component%20Object%20Reference) (OtherBodyIndex :type Integer) (bFromSweep :type Boolean) (SweepResult :type Hit%20Result%20Structure%20%28by%20ref%29))
  (if (== (Utilities|GetClass OtherActor) "/Game/ThirdPerson/Blueprints/BP_ThirdPersonCharacter.BP_ThirdPersonCharacter_C")
    (Utilities|FlowControl|DoOnce false
      (:Completed
        (Game|Damage|ApplyDamage OtherActor 1e+01 0 0)
        (Niagara|SpawnSystematLocation "/Game/P_Explosion.P_Explosion" (Transformation|GetActorLocation))
        (Actor|DestroyActor)))))

(event EventBeginPlay
  (bind _projectilemovement (Variables|Default|GetProjectileMovement))
  (Utilities|FlowControl|Delay 1.0)
  (Transformation|SetActorRotation (Math|Rotator|FindLookatRotation (Transformation|GetActorLocation) (Transformation|GetActorLocation (Game|Player|GetPlayerPawn 0))) true)
  (Components|Activation|Activate (Variables|Default|GetProjectileMovement) false)
  (Game|Components|ProjectileMovement|SetVelocityinLocalSpace _projectilemovement (Math|Vector|MakeVector (Variables|/Script/Engine.ProjectileMovementComponent|GetInitialSpeed _projectilemovement) 0.0 0.0)))

(fn ConstructionScript)