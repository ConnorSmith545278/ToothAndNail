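; BP_SlamArea is a growing slam area that marks stuck nails and detonates them when the slam ends.
; Grow uses a timeline to scale the root uniformly up one stage, while sphere overlaps collect BP_StuckNail actors.
; EndSlam removes the sphere and plane components, insertion-sorts nails by distance and staggers their explosions from farthest to nearest, then destroys the actor.
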(event OnComponentBeginOverlap(Sphere)
  (params (OverlappedComponent :type Primitive%20Component%20Object%20Reference) (OtherActor :type Actor%20Object%20Reference) (OtherComp :type Primitive%20Component%20Object%20Reference) (OtherBodyIndex :type Integer) (bFromSweep :type Boolean) (SweepResult :type Hit%20Result%20Structure%20%28by%20ref%29))
  (bind _asbp_stuck_nail (Utilities|Casting|CastToBP_StuckNail OtherActor))
  (Utilities|Array|Add (Variables|Default|GetMarkedNails) _asbp_stuck_nail))

(event Custom|Grow
  (params (ToStage :type Integer) (DiameterPerStage :type Float%20%28double-precision%29))
  (bind _returnvalue (- ToStage 1))
  (bind _returnvalue_2 (* ToStage DiameterPerStage))
  (bind _returnvalue_3 (* _returnvalue DiameterPerStage))
  (bind _newtrack_0 (Timeline|Grow%20Timeline PlayFromStart)
    (:Update
      (Transformation|SetWorldScale3D (Variables|Default|GetDefaultSceneRoot) (Math|Vector|Lerp(Vector) (Math|Vector|MakeVector _returnvalue_3 _returnvalue_3 _returnvalue_3) (Math|Vector|MakeVector _returnvalue_2 _returnvalue_2 _returnvalue_2) _newtrack_0)))))

(event Custom|EndSlam
  (Utilities|FlowControl|Sequence
    (:then_0
      (Components|DestroyComponent (Variables|Default|GetSphere1))
      (Components|DestroyComponent (Variables|Default|GetPlane)))
    (:then_1
      (bind _sortedarray (CallFunction|SortArraybyDistancefrom (Variables|Default|GetMarkedNails)))
      (bind (_arrayindex _arrayelement) (Utilities|Array|ReverseforEachLoop _sortedarray)
        (:LoopBody
          (Default|Explode _arrayelement (* 0.1 _arrayindex) 1.0))
        (:Completed
          (Development|PrintString "End")
          (Actor|DestroyActor))))))

(fn ConstructionScript)

(fn SortArraybyDistancefrom
  (params (Array :type Array%20of%20BP%20Stuck%20Nail%20Object%20References))
  (bind _output_get (LocalVariables|SetWorkingArray Array))
  (for _array_element _output_get
    (bind _asbp_stuck_nail (Utilities|Casting|CastToBP_StuckNail _array_element))
    (bind _output_get_2 (LocalVariables|SetCurrentActor _asbp_stuck_nail))
    (LocalVariables|SetCurrentDistance (Transformation|GetDistanceTo _output_get_2 self))
    (LocalVariables|SetInsertIndex (Utilities|Array|Length (LocalVariables|GetArraySorted)))
    (bind (_arrayindex _arrayelement) (Utilities|Array|ReverseforEachLoop (LocalVariables|GetArraySorted))
      (:LoopBody
        (if (< (Transformation|GetDistanceTo _arrayelement self) (LocalVariables|GetCurrentDistance))
          (LocalVariables|SetInsertIndex _arrayindex)))
      (:Completed
        (Utilities|Array|Insert (LocalVariables|GetArraySorted) (LocalVariables|GetCurrentActor) (LocalVariables|GetInsertIndex)))))
  (return (LocalVariables|GetArraySorted)))