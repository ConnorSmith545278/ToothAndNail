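; BP_PoisonTravelingNail is the in-flight poison nail projectile, which turns into a stuck nail on impact.
; When its Body hits anything other than the instigator or a Projectile-tagged actor, it spawns BP_PoisonStuckNail at the impact point with its own rotation.
; It attaches that nail to the hit component, keeping world transform, then destroys itself.
; An AC_Health impact-damage branch using StickDamage is present but never runs.
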(event OnComponentHit(Body)
  (params (HitComponent :type Primitive%20Component%20Object%20Reference) (OtherActor :type Actor%20Object%20Reference) (OtherComp :type Primitive%20Component%20Object%20Reference) (NormalImpulse :type Vector :default "0, 0, 0") (Hit :type Hit%20Result%20Structure%20%28by%20ref%29))
  (if (not (== OtherActor (Game|GetInstigator)))
    (if (not (Actor|ActorHasTag OtherActor "Projectile"))
      (bind _returnvalue (Game|SpawnActorfromClass "/Game/Blueprints/BP_PoisonStuckNail.BP_PoisonStuckNail_C" (Math|Transform|MakeTransform (.ImpactPoint (Collision|BreakHitResult Hit)) (Transformation|GetActorRotation self) "1.000000,1.000000,1.000000") "AlwaysSpawn" "MultiplyWithRoot" 0 0))
      (Transformation|AttachComponentToComponent _returnvalue OtherComp "None" "KeepWorld" "KeepWorld" "KeepWorld" true)
      (Actor|DestroyActor))))

(fn ConstructionScript)