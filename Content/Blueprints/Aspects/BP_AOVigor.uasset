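; BP_AOVigor is an aspect actor that boosts the player's damage in proportion to their current health.
; On BeginPlay it binds to the player character's health update event and recalculates the multiplier on each update, rising from 1.0 by half of MaxDamageMultiplier at full health.
; The result is written to the character, mirrored to GI_Game and printed.
; RemoveAspect resets both multipliers to 1.0 and destroys the actor.
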(event Custom|UpdateDamageMultiplier
  (params (CurrentHealth :type Float%20%28double-precision%29) (MaxHealth :type Float%20%28double-precision%29))
  (bind _output_get (Variables|/Game/ThirdPerson/Blueprints/BP_ThirdPersonCharacter.BP_ThirdPersonCharacter_C|SetTotalDamageMultiplier (stale EventBeginPlay _asbp_third_person_character) (+ (* (/ CurrentHealth MaxHealth) (Variables|Default|GetMaxDamageMultiplier) 0.5) 1.0)))
  (bind _asgi_game (Utilities|Casting|CastToGI_Game (Game|GetGameInstance)))
  (bind _output_get_2 (Variables|/Game/Blueprints/GameInstances/GI_Game.GI_Game_C|SetOverallDamageMultiplier _asgi_game _output_get))
  (Development|PrintString (Utilities|String|ToString(Float) _output_get_2)))

(event EventBeginPlay
  (bind _asbp_third_person_character (Utilities|Casting|CastToBP_ThirdPersonCharacter (Game|Player|GetPlayerPawn 0)))
  (EventDispatchers|BindEventtoEUpdateHealth _asbp_third_person_character (delegate Custom|UpdateDamageMultiplier))
  (CallFunction|UpdateDamageMultiplier (Variables|/Game/ThirdPerson/Blueprints/BP_ThirdPersonCharacter.BP_ThirdPersonCharacter_C|GetCurrentHealth _asbp_third_person_character) (Variables|/Game/ThirdPerson/Blueprints/BP_ThirdPersonCharacter.BP_ThirdPersonCharacter_C|GetMaxHealth _asbp_third_person_character)))

(event EventRemoveAspect
  (bind _asbp_third_person_character (Utilities|Casting|CastToBP_ThirdPersonCharacter (Game|Player|GetPlayerPawn 0)))
  (bind _output_get (Variables|/Game/ThirdPerson/Blueprints/BP_ThirdPersonCharacter.BP_ThirdPersonCharacter_C|SetTotalDamageMultiplier _asbp_third_person_character 1.0))
  (bind _asgi_game (Utilities|Casting|CastToGI_Game (Game|GetGameInstance)))
  (Variables|/Game/Blueprints/GameInstances/GI_Game.GI_Game_C|SetOverallDamageMultiplier _asgi_game _output_get)
  (Actor|DestroyActor))

(fn ConstructionScript
  (|CallParentFunction))