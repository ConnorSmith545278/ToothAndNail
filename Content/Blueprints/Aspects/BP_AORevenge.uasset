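; Revenge aspect actor that raises the player's damage multiplier as their health drops.
; On BeginPlay it binds to the player character's health update event, then scales the multiplier by max over current health, so a bonus applies even at full health.
; The result is mirrored to the game instance's overall multiplier.
; RemoveAspect resets both multipliers to 1 and destroys the actor.
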(event Custom|UpdateDamageMultiplier
  (params (CurrentHealth :type Float%20%28double-precision%29) (MaxHealth :type Float%20%28double-precision%29))
  (bind _output_get (Variables|/Game/ThirdPerson/Blueprints/BP_ThirdPersonCharacter.BP_ThirdPersonCharacter_C|SetTotalDamageMultiplier (stale EventBeginPlay _asbp_third_person_character) (+ (* (/ MaxHealth CurrentHealth) (Variables|Default|GetMaxDamageMultiplier) 0.1) 1.0)))
  (bind _asgi_game (Utilities|Casting|CastToGI_Game (Game|GetGameInstance)))
  (Variables|/Game/Blueprints/GameInstances/GI_Game.GI_Game_C|SetOverallDamageMultiplier _asgi_game _output_get))

(event EventBeginPlay
  (bind _asbp_third_person_character (Utilities|Casting|CastToBP_ThirdPersonCharacter (Game|Player|GetPlayerPawn 0)))
  (EventDispatchers|BindEventtoEUpdateHealth _asbp_third_person_character (delegate Custom|UpdateDamageMultiplier)))

(event EventRemoveAspect
  (bind _asbp_third_person_character (Utilities|Casting|CastToBP_ThirdPersonCharacter (Game|Player|GetPlayerPawn 0)))
  (bind _output_get (Variables|/Game/ThirdPerson/Blueprints/BP_ThirdPersonCharacter.BP_ThirdPersonCharacter_C|SetTotalDamageMultiplier _asbp_third_person_character 1.0))
  (bind _asgi_game (Utilities|Casting|CastToGI_Game (Game|GetGameInstance)))
  (Variables|/Game/Blueprints/GameInstances/GI_Game.GI_Game_C|SetOverallDamageMultiplier _asgi_game _output_get)
  (Actor|DestroyActor))

(fn ConstructionScript
  (|CallParentFunction))