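; BP_AOBalance is an aspect actor that grants the player a max health bonus while it exists.
; On BeginPlay it raises the third-person character's MaxHealth by a fixed amount, fills CurrentHealth to that maximum and triggers the health update call.
; RemoveAspect subtracts the same bonus, also sets health to the new maximum, refreshes it, then destroys the actor.
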(event EventBeginPlay
  (bind _asbp_third_person_character (Utilities|Casting|CastToBP_ThirdPersonCharacter (Game|Player|GetPlayerPawn 0)))
  (bind _output_get (Variables|/Game/ThirdPerson/Blueprints/BP_ThirdPersonCharacter.BP_ThirdPersonCharacter_C|SetMaxHealth _asbp_third_person_character (+ (Variables|/Game/ThirdPerson/Blueprints/BP_ThirdPersonCharacter.BP_ThirdPersonCharacter_C|GetMaxHealth _asbp_third_person_character) 5e+01)))
  (bind _output_get_2 (Variables|/Game/ThirdPerson/Blueprints/BP_ThirdPersonCharacter.BP_ThirdPersonCharacter_C|SetCurrentHealth _asbp_third_person_character (Variables|/Game/ThirdPerson/Blueprints/BP_ThirdPersonCharacter.BP_ThirdPersonCharacter_C|GetMaxHealth _asbp_third_person_character)))
  (Default|CallEUpdateHealth _asbp_third_person_character _output_get_2 _output_get))

(event EventRemoveAspect
  (bind _asbp_third_person_character (Utilities|Casting|CastToBP_ThirdPersonCharacter (Game|Player|GetPlayerPawn 0)))
  (bind _output_get (Variables|/Game/ThirdPerson/Blueprints/BP_ThirdPersonCharacter.BP_ThirdPersonCharacter_C|SetMaxHealth _asbp_third_person_character (+ (Variables|/Game/ThirdPerson/Blueprints/BP_ThirdPersonCharacter.BP_ThirdPersonCharacter_C|GetMaxHealth _asbp_third_person_character) -5e+01)))
  (bind _output_get_2 (Variables|/Game/ThirdPerson/Blueprints/BP_ThirdPersonCharacter.BP_ThirdPersonCharacter_C|SetCurrentHealth _asbp_third_person_character (Variables|/Game/ThirdPerson/Blueprints/BP_ThirdPersonCharacter.BP_ThirdPersonCharacter_C|GetMaxHealth _asbp_third_person_character)))
  (Default|CallEUpdateHealth _asbp_third_person_character _output_get_2 _output_get)
  (Actor|DestroyActor))

(fn ConstructionScript
  (|CallParentFunction))